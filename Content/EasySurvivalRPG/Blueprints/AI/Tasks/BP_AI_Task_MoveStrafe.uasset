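; AI behavior tree task that makes the controlled pawn strafe in short random moves while focused on the blackboard target actor.
; It runs a random number of moves with random pauses between them, then waits and finishes successfully.
; Each move trace-checks a diagonal offset from the pawn before calling AIMoveTo, storing the destination in the blackboard meanwhile.
; A blocked path flips direction and uses up a move without pausing.
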(event Custom|LoopStrafeMove
  (params (MovesRemaining :type Integer))
  (bind _returnvalue (- MovesRemaining 1))
  ;[1 1 1] One strafe move in the loop.
  (Utilities|MoveStrafe
    (:Success
      (Utilities|FlowControl|Delay (Math|Random|RandomFloatinRange (Variables|Settings|GetMinDelayBeetweenMoves) (Variables|Settings|GetMaxDelayBeetweenMoves)) :!label _label))
    (:Failed
      (goto _label))
    (:Blocked
      _))
  (if (> _returnvalue 0)
    (CallFunction|LoopStrafeMove _returnvalue)
    (else
      (Utilities|FlowControl|Delay (Math|Random|RandomFloatinRange (Variables|Settings|GetMinDelayAfterMoves) (Variables|Settings|GetMaxDelayAfterMoves)))
      (AI|BehaviorTree|FinishExecute true))))

(event EventReceiveExecuteAI
  (params (OwnerController :type AI%20Controller%20Object%20Reference) (ControlledPawn :type Pawn%20Object%20Reference))
  ;[1 1 1] Move strafe arount target actor.
  (Variables|State|SetOwnerController OwnerController)
  (Variables|State|SetControlledPawn ControlledPawn)
  (AI|SetFocus OwnerController (AI|BehaviorTree|GetBlackboardValueasActor (Variables|Blackboard|GetTargetActor)))
  (Variables|State|SetStrafeDirection (Math|Random|RandomBool))
  (bind _output_get (Variables|State|SetLoopMoves (Math|Random|RandomIntegerinRange 1 (Variables|Settings|GetMaxStrafeMoves))))
  (CallFunction|LoopStrafeMove _output_get))