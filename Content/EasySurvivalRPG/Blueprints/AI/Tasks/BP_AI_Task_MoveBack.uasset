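; Behavior tree task that makes an AI pawn retreat from its target actor while keeping focus on it.
; It picks a point at a random distance along the line between target and pawn, optionally snapped to a random reachable nearby point, and validates it with a path trace.
; A clear path triggers AI MoveTo with the destination mirrored to the blackboard.
; Every outcome, including blocked, finishes as success, with optional short random delays.
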(event EventReceiveExecuteAI
  (params (OwnerController :type AI%20Controller%20Object%20Reference) (ControlledPawn :type Pawn%20Object%20Reference))
  ;[1 1 1] Move back from target actor.
  (bind _output_get (Variables|State|SetOwnerController OwnerController))
  (Variables|State|SetControlledPawn ControlledPawn)
  (AI|SetFocus _output_get (AI|BehaviorTree|GetBlackboardValueasActor (Variables|Blackboard|GetTargetActor)))
  (Utilities|MoveBack
    (:Success
      (if (Variables|Settings|GetDelayBeetweenMoves) :!label _label
        (Utilities|FlowControl|Delay (Math|Random|RandomFloatinRange 0.3 0.5))))
    (:Failed
      (goto _label))
    (:Blocked
      _))
  (AI|BehaviorTree|FinishExecute true))