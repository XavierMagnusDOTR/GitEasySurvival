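; Behavior tree task that makes an AI pawn run away from the actor stored in the TargetActor blackboard key.
; It offsets a point by a negated random distance between DistanceMin and DistanceMax along the pawn-to-target line, then picks a random reachable location near it.
; AIMoveTo sends the pawn there, and the task finishes as successful even when the move fails or the target is invalid.
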(event EventReceiveExecuteAI
  (params (OwnerController :type AI%20Controller%20Object%20Reference) (ControlledPawn :type Pawn%20Object%20Reference))
  (bind _targetactor (Variables|Blackboard|GetTargetActor))
  (bind _returnvalue (AI|BehaviorTree|GetBlackboardValueasActor _targetactor))
  ;[1 1 1] Try to run away from Target Actor.
  (Utilities|IsValid _returnvalue
    (:Is%20Valid
      (AI|AIMoveTo ControlledPawn (.RandomLocation (AI|Navigation|GetRandomReachablePointinRadius (CallFunction|GetLocationBetweenActors ControlledPawn _returnvalue (* (Math|Random|RandomFloatinRange (Variables|Default|GetDistanceMin) (Variables|Default|GetDistanceMax)) -1.0)) 1e+02 0 0)) 0 (Variables|Default|GetAcceptanceRadius) false
        (:OnSuccess
          (AI|BehaviorTree|FinishExecute true))
        (:OnFail
          (AI|BehaviorTree|FinishExecute true :!label _label))))
    (:Is%20Not%20Valid
      (goto _label))))