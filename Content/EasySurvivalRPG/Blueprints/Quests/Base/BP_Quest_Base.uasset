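; Base quest actor that runs a staged quest for one player, with child classes defining stages and their task components.
; Start, completion and failure add gameplay tags to the player controller; completion and failure also destroy the actor.
; Task events push progress to the controller, and a stage completes when a main task or all tasks finish.
; Task progress is saved as a semicolon-delimited string and restored by array index.
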(fn ConstructionScript)

(fn StartQuest
  ;[1 1 1] Start quest and add start tags for player.
  (Class|BPIPlayer|AddGameplayTagsBPI(Message) (Variables|/Game/EasySurvivalRPG/Blueprints/Components/BP_PlayerManagerComponent.BP_PlayerManagerComponent_C|GetPlayerController (Variables|State|GetPlayerManagerComponent)) (Variables|Settings|GetStartQuestTags))
  (Quest|StartQuestStage (Variables|Settings|GetDefaultQuestStage)))

(fn StartQuestStage
  (params (Stage :type Name))
  ;[1 1 1] Start quest stage and init stage tasks. Overridden in child class.
  (Quest|InitQuestStage Stage)
  (Quest|UpdateQuestProgress))

(fn CompleteQuest
  ;[1 1 1] Complete quest, add complete tags for player and destroy quest actor.
  (Class|BPIPlayer|AddGameplayTagsBPI(Message) (Variables|/Game/EasySurvivalRPG/Blueprints/Components/BP_PlayerManagerComponent.BP_PlayerManagerComponent_C|GetPlayerController (Variables|State|GetPlayerManagerComponent)) (Variables|Settings|GetCompleteQuestTags))
  (Default|CallOnCompleted self)
  (Actor|DestroyActor))

(fn InitQuestStage
  (params (Stage :type Name))
  ;[1 1 1] Set current quest stage and init tasks for the stage. Overridden in child class.
  (Variables|State|SetCurrentQuestStage Stage))

(fn InitQuest
  (params (PlayerManagerComponent :type BP%20Player%20Manager%20Component%20Object%20Reference))
  ;[1 1 1] Init quest and set references.
  (Variables|State|SetPlayerManagerComponent PlayerManagerComponent))

(fn UpdateQuestProgress
  (bind (_progress _progresstext) (Quest|GetQuestProgress))
  ;[1 1 1] Update quest progress for the player.
  (Class|BPIPlayer|UpdateQuestProgressBPI(Message) (Variables|/Game/EasySurvivalRPG/Blueprints/Components/BP_PlayerManagerComponent.BP_PlayerManagerComponent_C|GetPlayerController (Variables|State|GetPlayerManagerComponent)) (Variables|Settings|GetQuestID) (Variables|State|GetCurrentQuestStage) _progress _progresstext))

(fn GetQuestProgress
  ;[1 1 1] Get quest progress and progress text from active quest tasks.
  (for _array_element (Variables|State|GetActiveTasks)
    (LocalVariables|SetLocalProgress (Utilities|String|Append (LocalVariables|GetLocalProgress) (Default|GetProgress _array_element) ";"))
    (LocalVariables|SetLocalProgressText (select (Utilities|Text|TextIsEmpty (LocalVariables|GetLocalProgressText)) (Default|GetProgressText _array_element) (Utilities|Text|FormatText "{LocalText} 
{NewText}" (LocalVariables|GetLocalProgressText) (Default|GetProgressText _array_element)))))
  (return (LocalVariables|GetLocalProgress) (LocalVariables|GetLocalProgressText)))

(fn LoadQuestProgress
  (params (Progress :type String))
  ;[1 1 1] Load quest progress for active tasks.
  (bind _output_get (LocalVariables|SetLocalProgress (Utilities|String|ParseIntoArray Progress ";")))
  (for (_array_element _array_index) (Variables|State|GetActiveTasks)
    (Default|LoadProgress _array_element (Utilities|Array|Get(acopy) _output_get _array_index))))

(fn FailQuest
  ;[1 1 1] Fail quest and add fail quest tags for player.
  (Class|BPIPlayer|AddGameplayTagsBPI(Message) (Variables|/Game/EasySurvivalRPG/Blueprints/Components/BP_PlayerManagerComponent.BP_PlayerManagerComponent_C|GetPlayerController (Variables|State|GetPlayerManagerComponent)) (Variables|Settings|GetFailQuestTags))
  (Default|CallOnFailed self)
  (Actor|DestroyActor))

(fn TaskCompleted
  (params (QuestTaskComponent :type BP%20Quest%20Task%20Component%20Base%20Object%20Reference))
  (bind _activetasks (Variables|State|GetActiveTasks))
  ;[1 1 1] Event when task was completed. Check active tasks and complete quest if all tasks completed.
  (if (Utilities|Array|ContainsItem _activetasks QuestTaskComponent)
    (for _array_element _activetasks
      (if (and (Variables|/Game/EasySurvivalRPG/Blueprints/Components/QuestTasks/BP_QuestTaskComponent_Base.BP_QuestTaskComponent_Base_C|GetMainTask _array_element) (Variables|/Game/EasySurvivalRPG/Blueprints/Components/QuestTasks/BP_QuestTaskComponent_Base.BP_QuestTaskComponent_Base_C|GetIsCompleted _array_element))
        (Quest|CompleteQuestStage (Variables|State|GetCurrentQuestStage))
        (return)))
    (for _array_element_2 _activetasks
      (if (not (Variables|/Game/EasySurvivalRPG/Blueprints/Components/QuestTasks/BP_QuestTaskComponent_Base.BP_QuestTaskComponent_Base_C|GetIsCompleted _array_element_2))
        (return)))
    (Quest|CompleteQuestStage (Variables|State|GetCurrentQuestStage))))

(fn TaskProgressChanged
  (params (QuestTaskComponent :type BP%20Quest%20Task%20Component%20Base%20Object%20Reference))
  ;[1 1 1] Event when task progress was changed.
  (if (Utilities|Array|ContainsItem (Variables|State|GetActiveTasks) QuestTaskComponent)
    (Quest|UpdateQuestProgress)))

(fn CompleteQuestStage
  (params (Stage :type Name))
  ;[1 1 1] Complete quest stage. Overridden in child class.
)

(fn ClearTasks
  (bind _activetasks (Variables|State|GetActiveTasks))
  ;[1 1 1] Clear and destroy active quest tasks components.
  (for _array_element _activetasks
    (Components|DestroyComponent _array_element))
  (Utilities|Array|Clear _activetasks))

(fn InitTasks
  (params (Tasks :type Array%20of%20BP%20Quest%20Task%20Component%20Base%20Object%20References))
  ;[1 1 1] Init target quest tasks components.
  (bind _output_get (Variables|State|SetActiveTasks Tasks))
  (for _array_element _output_get
    (EventDispatchers|BindEventtoOnCompleted _array_element (EventDispatchers|CreateEvent :!event TaskCompleted))
    (EventDispatchers|BindEventtoOnFailed _array_element (EventDispatchers|CreateEvent :!event TaskFailed))
    (EventDispatchers|BindEventtoOnProgressUpdated _array_element (EventDispatchers|CreateEvent :!event TaskProgressChanged))
    (Default|InitComponent _array_element (Variables|State|GetPlayerManagerComponent))))

(fn TaskFailed
  (params (QuestTaskComponent :type BP%20Quest%20Task%20Component%20Base%20Object%20Reference))
  ;[1 1 1] Event when quest task was failed.
  (Default|CallOnFailed self))