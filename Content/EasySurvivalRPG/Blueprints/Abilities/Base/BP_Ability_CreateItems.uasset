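; Base ability actor that creates items and gives them to the character that used it.
; On Use it builds loot items from the first effect in its ability settings, falling back to ItemsToCreateHandle when none is set.
; It adds them through the inventory container fetched from the instigator's controller by interface message, with a drop fallback, then destroys itself.
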(event EventUse
  ;[1 1 1] Try to add items to instigator's inventory.
  (Utilities|FlowControl|Sequence
    (:then_0
      (Ability|AddItemstoCharacter))
    (:then_1
      (Actor|DestroyActor))))

(fn ConstructionScript
  (|CallParentFunction))

(fn AddItemstoCharacter
  (bind _abilitysettings (Variables|Default|GetAbilitySettings))
  (bind _effects (Utilities|Struct|BreakSTR_AbilityInstance _abilitysettings))
  ;[1 1 1] Add items to the instigator's inventory component.
  (bind _inventorycontainer (Class|BPIPlayer|GetInventoryContainerBPI(Message) (Game|GetInstigatorController)))
  (Default|TryAddItemsorDrop _inventorycontainer (CallFunction|MakeLootItems (select (Utilities|Array|IsValidIndex _effects) (Utilities|Array|Get(acopy) _effects) (Variables|Settings|GetItemsToCreateHandle)))))