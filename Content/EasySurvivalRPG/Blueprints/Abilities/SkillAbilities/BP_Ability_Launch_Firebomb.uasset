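; Firebomb launch skill ability that spawns one or more projectiles from the instigator's weapon socket toward where they are aiming.
; SpawnProjectile falls back to above the actor if the socket location is zero, then traces from the controller's focus point to set the launch rotation.
; The first projectile flies true while extras get random pitch and yaw spread.
; LaunchProjectile spawns each with the ability's attributes, optionally updating them from the instigator.
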(event EventBeginPlay)

(event Collision|EventActorBeginOverlap
  (params (OtherActor :type Actor%20Object%20Reference)))

(event EventTick
  (params (DeltaSeconds :type Float%20%28single-precision%29)))

(fn ConstructionScript
  (|CallParentFunction))

(fn SpawnProjectile
  (bind _returnvalue (Game|GetInstigator))
  (Utilities|IsValid _returnvalue
    (:Is%20Valid
      (bind _sockettransform (Class|BPICharacter|GetWeaponSocketTransformBPI(Message) _returnvalue (Variables|Default|GetWeaponStartSocketName)))
      (LocalVariables|SetLocalStartLocation (select (Math|Vector|Equal(Vector) (.Location (Math|Transform|BreakTransform _sockettransform)) "0, 0, 0" 0.0001) (+ (Transformation|GetActorLocation _returnvalue) "0, 0,100.000000") (.Location (Math|Transform|BreakTransform _sockettransform))))
      (bind (_location _rotation) (CallFunction|GetFocusVariables (Game|GetInstigatorController)))
      (bind (_washit _hitlocation) (CallFunction|GetTraceHitLocation _location _rotation 1e+04))
      (if _washit
        (bind _output_get (LocalVariables|SetLocalTraceHitLocation _hitlocation))
        (LocalVariables|SetLocalRotation (Math|Rotator|FindLookatRotation (LocalVariables|GetLocalStartLocation) _output_get))
        (else
          (LocalVariables|SetLocalRotation (Math|Rotator|FindLookatRotation (LocalVariables|GetLocalStartLocation) (+ _location (* (Math|Vector|GetForwardVector _rotation) 1e+04))))))
      (for _index (range 0 (- (Variables|Settings|Projectile|GetProjectilesCount) 1))
        (CallFunction|LaunchProjectile (LocalVariables|GetLocalStartLocation) (select (> _index 0) (Math|Rotator|CombineRotators (LocalVariables|GetLocalRotation) (Math|Rotator|MakeRotator 0.0 (Math|Random|RandomFloatinRange -5.0 5.0) (Math|Random|RandomFloatinRange -5.0 5.0))) (LocalVariables|GetLocalRotation)) (Variables|Default|GetProjectileScale))))
    (:Is%20Not%20Valid
      (return false))))

(fn LaunchProjectile
  (params (StartLocation :type Vector) (Rotation :type Rotator) (Scale :type Vector :default "1.000000,1.000000,1.000000"))
  ;[1 1 1] Spawn and launch projectile by specific class to target direction.
  (bind _returnvalue (Game|SpawnActorfromClass (Variables|Default|GetProjectileClass) (Math|Transform|MakeTransform StartLocation Rotation Scale) "Undefined" 0 (Utilities|Struct|BreakSTR_AbilityInstance (Variables|Default|GetAbilitySettings)) (Game|GetInstigator)))
  (if (Variables|Default|GetUseInstigatorAttributes)
    (Default|UpdateProjectileAttributes _returnvalue))
  (return true))