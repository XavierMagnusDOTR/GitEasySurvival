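; Trace-based skill ability that calls down a volley of meteor projectiles from the sky onto the traced hit location.
; A blocking hit picks a random offset spawn point high above the target, aims at it, and starts a looping timer to stagger the launches.
; SpawnMeteor fires each projectile with slight random pitch and yaw spread, passing along ability attributes, and destroys the ability actor once the count runs out.
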(fn ConstructionScript
  (|CallParentFunction))

(fn CheckHit
  (params (HitResult :type Hit%20Result%20Structure))
  (bind (_bblockinghit _binitialoverlap _time _distance _location) (Collision|BreakHitResult HitResult))
  (bind _meteorscount (Variables|Settings|Projectile|GetMeteorsCount))
  ;[1 1 1] Check trace hit result and spawn projectile.
  (if _bblockinghit
    (bind _output_get (LocalVariables|SetLocalHitLocation _location))
    (bind _output_get_2 (LocalVariables|SetLocalSpawnLocation (+ _output_get (Math|Vector|MakeVector (* (Math|Random|RandomFloatinRange 3e+03 5e+03) (Math|Random|RandomFloatinRange -1.0 1.0)) (* (Math|Random|RandomFloatinRange 3e+03 5e+03) (Math|Random|RandomFloatinRange -1.0 1.0)) 1e+04))))
    (Variables|State|SetSpawnLocation _output_get_2)
    (Variables|State|SetSpawnRotation (Math|Rotator|FindLookatRotation (LocalVariables|GetLocalSpawnLocation) _output_get))
    (Variables|State|SetCountRemaining _meteorscount)
    (Variables|State|SetMeteorIndex (/ _meteorscount 2))
    (Utilities|Time|SetTimerbyEvent (EventDispatchers|CreateEvent :!event SpawnMeteor) 0.125 true)
    (return true)))

(fn CheckAbilityConditions
  ;[1 1 1] Check ability cost and trace hit.
  (bind _success (|CallParentFunction))
  (if _success
    (CallFunction|UpdateTraceVariables)
    (bind _washit (CallFunction|TryHitTrace))
    (return _washit)
    (else
      (return _success))))

(fn UpdateTraceVariables
  (bind _abilitysettings (Variables|Default|GetAbilitySettings))
  (bind _attributes (Utilities|Struct|BreakSTR_AbilityInstance _abilitysettings))
  (bind (_success _value) (CallFunction|GetAttributeValue _attributes "(TagName=\"EasyRPG.Attributes.AbilitySystem.Projectile.Speed\")"))
  ;[1 1 1] Update trace variables.
  (bind _success_2 (|CallParentFunction))
  (Utilities|FlowControl|Sequence
    (:then_0
      (if _success
        (Variables|Settings|Projectile|SetProjectileSpeed _value)))
    (:then_1
      (return _success_2))))

(fn LaunchProjectile
  (params (ProjectileClass :type BP%20Projectile%20Base%20Class%20Reference) (StartLocation :type Vector) (Rotation :type Rotator) (Scale :type Vector :default "1.000000,1.000000,1.000000"))
  ;[1 1 1] Spawn and launch projectile by specific class with target direction.
  (bind _returnvalue (Game|SpawnActorfromClass ProjectileClass (Math|Transform|MakeTransform StartLocation Rotation Scale) "Undefined" 0 (Utilities|Struct|BreakSTR_AbilityInstance (Variables|Default|GetAbilitySettings)) (Game|GetInstigator)))
  (if (Variables|Settings|Projectile|GetUseInstigatorAttributes)
    (Default|UpdateProjectileAttributes _returnvalue))
  (return true))

(fn SpawnMeteor
  ;[1 1 1] Spawn meteor from the sky.
  (if (> (Variables|State|GetCountRemaining) 0)
    (Variables|State|SetCountRemaining (- (Variables|State|GetCountRemaining) 1))
    (Ability|LaunchProjectile (Variables|Settings|Projectile|GetProjectileClass) (Variables|State|GetSpawnLocation) (Math|Rotator|CombineRotators (Variables|State|GetSpawnRotation) (Math|Rotator|MakeRotator 0.0 (Math|Random|RandomFloatinRange -5.0 5.0) (Math|Random|RandomFloatinRange -5.0 5.0))) (Variables|Settings|Projectile|GetProjectileScale))
    (else
      (Actor|DestroyActor))))