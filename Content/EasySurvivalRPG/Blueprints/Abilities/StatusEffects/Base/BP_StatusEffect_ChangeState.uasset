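; Base status effect that drains or restores its owner's health, energy, hunger, thirst, oxygen and mana over time.
; UpdateVariables reads flat and percent per-second rates from the effect settings' gameplay-tagged attributes.
; Each tick, TickActions applies non-zero rates, scaled by delta time and stack count, through Blueprint interface messages to the owner.
; The effect destroys itself when the owner is no longer alive.
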(fn ConstructionScript
  (|CallParentFunction))

(fn UpdateVariables
  (bind _effectsettings (Variables|Default|GetEffectSettings))
  (bind _effectattributes (Utilities|Struct|BreakSTR_StatusEffectInstance _effectsettings))
  ;[1 1 1] Update status effect variables.
  (bind _success (|CallParentFunction))
  (if (Utilities|Array|IsValidIndex _effectattributes)
    (LocalVariables|SetLocalAttributes _effectattributes)
    (Utilities|FlowControl|Sequence
      (:then_0
        (Utilities|FlowControl|Sequence
          (:then_0
            (if (.Success (CallFunction|GetAttributeValue (LocalVariables|GetLocalAttributes) "(TagName=\"EasyRPG.Attributes.StatusEffect.Health.ValuePerSecond\")"))
              (Variables|Settings|SetHealthPerSecond (.Value (CallFunction|GetAttributeValue (LocalVariables|GetLocalAttributes) "(TagName=\"EasyRPG.Attributes.StatusEffect.Health.ValuePerSecond\")")))))
          (:then_1
            (if (.Success (CallFunction|GetAttributeValue (LocalVariables|GetLocalAttributes) "(TagName=\"EasyRPG.Attributes.StatusEffect.Health.Max%PerSecond\")"))
              (Variables|Settings|SetHealthPercentPerSecond (.Value (CallFunction|GetAttributeValue (LocalVariables|GetLocalAttributes) "(TagName=\"EasyRPG.Attributes.StatusEffect.Health.Max%PerSecond\")")))))))
      (:then_1
        (Utilities|FlowControl|Sequence
          (:then_0
            (if (.Success (CallFunction|GetAttributeValue (LocalVariables|GetLocalAttributes) "(TagName=\"EasyRPG.Attributes.StatusEffect.Energy.ValuePerSecond\")"))
              (Variables|Settings|SetEnergyPerSecond (.Value (CallFunction|GetAttributeValue (LocalVariables|GetLocalAttributes) "(TagName=\"EasyRPG.Attributes.StatusEffect.Energy.ValuePerSecond\")")))))
          (:then_1
            (if (.Success (CallFunction|GetAttributeValue (LocalVariables|GetLocalAttributes) "(TagName=\"EasyRPG.Attributes.StatusEffect.Energy.Max%PerSecond\")"))
              (Variables|Settings|SetEnergyPercentPerSecond (.Value (CallFunction|GetAttributeValue (LocalVariables|GetLocalAttributes) "(TagName=\"EasyRPG.Attributes.StatusEffect.Energy.Max%PerSecond\")")))))))
      (:then_2
        (Utilities|FlowControl|Sequence
          (:then_0
            (if (.Success (CallFunction|GetAttributeValue (LocalVariables|GetLocalAttributes) "(TagName=\"EasyRPG.Attributes.StatusEffect.Hunger.ValuePerSecond\")"))
              (Variables|Settings|SetHungerPerSecond (.Value (CallFunction|GetAttributeValue (LocalVariables|GetLocalAttributes) "(TagName=\"EasyRPG.Attributes.StatusEffect.Hunger.ValuePerSecond\")")))))
          (:then_1
            (if (.Success (CallFunction|GetAttributeValue (LocalVariables|GetLocalAttributes) "(TagName=\"EasyRPG.Attributes.StatusEffect.Hunger.Max%PerSecond\")"))
              (Variables|Settings|SetHungerPercentPerSecond (.Value (CallFunction|GetAttributeValue (LocalVariables|GetLocalAttributes) "(TagName=\"EasyRPG.Attributes.StatusEffect.Hunger.Max%PerSecond\")")))))))
      (:then_3
        (Utilities|FlowControl|Sequence
          (:then_0
            (if (.Success (CallFunction|GetAttributeValue (LocalVariables|GetLocalAttributes) "(TagName=\"EasyRPG.Attributes.StatusEffect.Thirst.ValuePerSecond\")"))
              (Variables|Settings|SetThirstPerSecond (.Value (CallFunction|GetAttributeValue (LocalVariables|GetLocalAttributes) "(TagName=\"EasyRPG.Attributes.StatusEffect.Thirst.ValuePerSecond\")")))))
          (:then_1
            (if (.Success (CallFunction|GetAttributeValue (LocalVariables|GetLocalAttributes) "(TagName=\"EasyRPG.Attributes.StatusEffect.Thirst.Max%PerSecond\")"))
              (Variables|Settings|SetThirstPercentPerSecond (.Value (CallFunction|GetAttributeValue (LocalVariables|GetLocalAttributes) "(TagName=\"EasyRPG.Attributes.StatusEffect.Thirst.Max%PerSecond\")")))))))
      (:then_4
        (Utilities|FlowControl|Sequence
          (:then_0
            (if (.Success (CallFunction|GetAttributeValue (LocalVariables|GetLocalAttributes) "(TagName=\"EasyRPG.Attributes.StatusEffect.Oxygen.ValuePerSecond\")"))
              (Variables|Settings|SetOxygenPerSecond (.Value (CallFunction|GetAttributeValue (LocalVariables|GetLocalAttributes) "(TagName=\"EasyRPG.Attributes.StatusEffect.Oxygen.ValuePerSecond\")")))))
          (:then_1
            (if (.Success (CallFunction|GetAttributeValue (LocalVariables|GetLocalAttributes) "(TagName=\"EasyRPG.Attributes.StatusEffect.Oxygen.Max%PerSecond\")"))
              (Variables|Settings|SetOxygenPercentPerSecond (.Value (CallFunction|GetAttributeValue (LocalVariables|GetLocalAttributes) "(TagName=\"EasyRPG.Attributes.StatusEffect.Oxygen.Max%PerSecond\")")))))))
      (:then_5
        (Utilities|FlowControl|Sequence
          (:then_0
            (if (.Success (CallFunction|GetAttributeValue (LocalVariables|GetLocalAttributes) "(TagName=\"EasyRPG.Attributes.StatusEffect.Mana.ValuePerSecond\")"))
              (Variables|Settings|SetManaPerSecond (.Value (CallFunction|GetAttributeValue (LocalVariables|GetLocalAttributes) "(TagName=\"EasyRPG.Attributes.StatusEffect.Mana.ValuePerSecond\")")))))
          (:then_1
            (if (.Success (CallFunction|GetAttributeValue (LocalVariables|GetLocalAttributes) "(TagName=\"EasyRPG.Attributes.StatusEffect.Mana.Max%PerSecond\")"))
              (Variables|Settings|SetManaPercentPerSecond (.Value (CallFunction|GetAttributeValue (LocalVariables|GetLocalAttributes) "(TagName=\"EasyRPG.Attributes.StatusEffect.Mana.Max%PerSecond\")")))))))
      (:then_6
        (return _success)))
    (else
      (return _success))))

(fn CheckandChangeHealth
  (params (DeltaSecond :type Float%20%28single-precision%29))
  (bind _returnvalue (Components|GetOwner))
  (bind _healthpersecond (Variables|Settings|GetHealthPerSecond))
  (bind _healthpercentpersecond (Variables|Settings|GetHealthPercentPerSecond))
  (bind _stack (Variables|Default|GetStack))
  (bind _returnvalue_2 (Math|Conversions|ToFloat(Integer) _stack))
  ;[1 1 1] Change the owner's health state.
  (if (or (!= _healthpersecond 0.0) (!= _healthpercentpersecond 0.0))
    (Class|BPICharacter|ChangeHealthBPI(Message) _returnvalue (* _healthpersecond DeltaSecond _returnvalue_2) false)
    (Class|BPICharacter|ChangeHealthBPI(Message) _returnvalue (* _healthpercentpersecond DeltaSecond _returnvalue_2) true)))

(fn CheckandChangeEnergy
  (params (DeltaSecond :type Float%20%28single-precision%29))
  (bind _returnvalue (Components|GetOwner))
  (bind _energypersecond (Variables|Settings|GetEnergyPerSecond))
  (bind _energypercentpersecond (Variables|Settings|GetEnergyPercentPerSecond))
  (bind _stack (Variables|Default|GetStack))
  (bind _returnvalue_2 (Math|Conversions|ToFloat(Integer) _stack))
  ;[1 1 1] Change the owner's energy state.
  (if (or (!= _energypersecond 0.0) (!= _energypercentpersecond 0.0))
    (Class|BPICharacter|ChangeEnergyBPI(Message) _returnvalue (* _energypersecond DeltaSecond _returnvalue_2) false)
    (Class|BPICharacter|ChangeEnergyBPI(Message) _returnvalue (* _energypercentpersecond DeltaSecond _returnvalue_2) true)))

(fn CheckandChangeHunger
  (params (DeltaSecond :type Float%20%28single-precision%29))
  (bind _returnvalue (Components|GetOwner))
  (bind _hungerpersecond (Variables|Settings|GetHungerPerSecond))
  (bind _hungerpercentpersecond (Variables|Settings|GetHungerPercentPerSecond))
  (bind _stack (Variables|Default|GetStack))
  (bind _returnvalue_2 (Math|Conversions|ToFloat(Integer) _stack))
  ;[1 1 1] Change the owner's hunger state.
  (if (or (!= _hungerpersecond 0.0) (!= _hungerpercentpersecond 0.0))
    (Class|BPIPlayerCharacter|ChangeHungerBPI(Message) _returnvalue (* _hungerpersecond DeltaSecond _returnvalue_2) false)
    (Class|BPIPlayerCharacter|ChangeHungerBPI(Message) _returnvalue (* _hungerpercentpersecond DeltaSecond _returnvalue_2) true)))

(fn CheckandChangeThirst
  (params (DeltaSecond :type Float%20%28single-precision%29))
  (bind _returnvalue (Components|GetOwner))
  (bind _thirstpersecond (Variables|Settings|GetThirstPerSecond))
  (bind _thirstpercentpersecond (Variables|Settings|GetThirstPercentPerSecond))
  (bind _stack (Variables|Default|GetStack))
  (bind _returnvalue_2 (Math|Conversions|ToFloat(Integer) _stack))
  ;[1 1 1] Change the owner's thirst state.
  (if (or (!= _thirstpersecond 0.0) (!= _thirstpercentpersecond 0.0))
    (Class|BPIPlayerCharacter|ChangeThirstBPI(Message) _returnvalue (* _thirstpersecond DeltaSecond _returnvalue_2) false)
    (Class|BPIPlayerCharacter|ChangeThirstBPI(Message) _returnvalue (* _thirstpercentpersecond DeltaSecond _returnvalue_2) true)))

(fn CheckandChangeOxygen
  (params (DeltaSecond :type Float%20%28single-precision%29))
  (bind _returnvalue (Components|GetOwner))
  (bind _oxygenpersecond (Variables|Settings|GetOxygenPerSecond))
  (bind _oxygenpercentpersecond (Variables|Settings|GetOxygenPercentPerSecond))
  (bind _stack (Variables|Default|GetStack))
  (bind _returnvalue_2 (Math|Conversions|ToFloat(Integer) _stack))
  ;[1 1 1] Change the owner's oxygen state.
  (if (or (!= _oxygenpersecond 0.0) (!= _oxygenpercentpersecond 0.0))
    (Class|BPIPlayerCharacter|ChangeOxygenBPI(Message) _returnvalue (* _oxygenpersecond DeltaSecond _returnvalue_2) false)
    (Class|BPIPlayerCharacter|ChangeOxygenBPI(Message) _returnvalue (* _oxygenpercentpersecond DeltaSecond _returnvalue_2) true)))

(fn TickActions
  (params (DeltaSecond :type Float%20%28single-precision%29))
  ;[1 1 1] Change owner's state by tick.
  (bind _result (Class|BPICharacter|IsAliveBPI(Message) (Components|GetOwner)))
  (if _result
    (ChangeState|CheckandChangeHealth DeltaSecond)
    (ChangeState|CheckandChangeEnergy DeltaSecond)
    (ChangeState|CheckandChangeHunger DeltaSecond)
    (ChangeState|CheckandChangeThirst DeltaSecond)
    (ChangeState|CheckandChangeOxygen DeltaSecond)
    (ChangeState|CheckandChangeMana DeltaSecond)
    (bind _success (|CallParentFunction DeltaSecond))
    (return _success)
    (else
      (Actor|DestroyActor)
      (return true))))

(fn CheckandChangeMana
  (params (DeltaSecond :type Float%20%28single-precision%29))
  (bind _returnvalue (Components|GetOwner))
  (bind _manapersecond (Variables|Settings|GetManaPerSecond))
  (bind _manapercentpersecond (Variables|Settings|GetManaPercentPerSecond))
  (bind _stack (Variables|Default|GetStack))
  (bind _returnvalue_2 (Math|Conversions|ToFloat(Integer) _stack))
  ;[1 1 1] Change the owner's oxygen state.
  (if (or (!= _manapersecond 0.0) (!= _manapercentpersecond 0.0))
    (Class|BPICharacter|ChangeManaBPI(Message) _returnvalue (* _manapersecond DeltaSecond _returnvalue_2) false)
    (Class|BPICharacter|ChangeManaBPI(Message) _returnvalue (* _manapercentpersecond DeltaSecond _returnvalue_2) true)))