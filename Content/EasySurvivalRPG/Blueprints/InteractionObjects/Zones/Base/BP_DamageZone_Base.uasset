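; Base damage zone actor that hurts characters inside it, exists only on the authority and destroys itself on remote machines.
; AddOverlappingCharacter tracks characters, optionally only player-controlled ones, and deals immediate overlap damage while the zone is activated.
; Tick applies per-second damage scaled by delta time at a configurable interval, with activation toggling actor tick.
; Both paths send damage type, critical, block-break, interrupt and reaction settings through ApplyAdvancedPointDamage.
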(event EventTick
  (params (DeltaSeconds :type Float%20%28single-precision%29))
  ;[1 1 1] Event tick. Damage characters by tick if activated.
  (if (and (Variables|State|GetIsActivated) (Variables|State|GetUpdateStatesByTick))
    (for _array_element (Variables|State|GetOverlappingCharacters)
      (CallFunction|DamageCharacterbyTick _array_element DeltaSeconds))))

(event EventBeginPlay
  ;[1 1 1] Begin play. Set activated state.
  (Networking|SwitchHasAuthority
    (:Authority
      (CallFunction|SetActivatedState (Variables|Settings|GetInitiallyActivated)))
    (:Remote
      (Actor|DestroyActor))))

(fn ConstructionScript
  ;[1 1 1] Set tick variables variables.
  (Variables|State|SetUpdateStatesByTick (!= (Variables|Settings|TickDamage|GetTickDamagePerSecond) 0.0))
  (Actor|Tick|SetActorTickInterval (Variables|Settings|GetTickInterval)))

(fn AddOverlappingCharacter
  (params (Character :type Character%20Object%20Reference))
  ;[1 1 1] Add character to the overlapping characters array and damage it.
  (if (Variables|Settings|GetOnlyPlayerCharacters)
    (Utilities|Casting|CastToPlayerController (Pawn|GetController Character)))
  (Utilities|Array|AddUnique (Variables|State|GetOverlappingCharacters) Character)
  (CallFunction|DamageCharacterbyOverlap Character)
  (return true))

(fn RemoveOverlappingCharacter
  (params (Character :type Character%20Object%20Reference))
  ;[1 1 1] Remove character from overlapping characters array.
  (Utilities|Array|RemoveItem (Variables|State|GetOverlappingCharacters) Character)
  (return true))

(fn DamageCharacterbyOverlap
  (params (Character :type Character%20Object%20Reference))
  ;[1 1 1] Damage character on overlap event.
  (LocalVariables|SetLocalCharacter Character)
  (if (Variables|State|GetIsActivated)
    (CallFunction|DamageCharacter (LocalVariables|GetLocalCharacter) (Variables|Settings|OverlapDamage|GetOverlapDamage) (Variables|Settings|OverlapDamage|GetOverlapDamageType) (Variables|Settings|OverlapDamage|GetOverlapCriticalHit) (Variables|Settings|OverlapDamage|GetOverlapBreakBlock) (Variables|Settings|OverlapDamage|GetOverlapInterruptAnimation) (Variables|Settings|OverlapDamage|GetOverlapPlayerReactionEffects))
    (return true)))

(fn DamageCharacterbyTick
  (params (Character :type Character%20Object%20Reference) (DeltaSeconds :type Float%20%28single-precision%29))
  ;[1 1 1] Damage character by event tick.
  (LocalVariables|SetLocalCharacter Character)
  (LocalVariables|SetLocalDeltaSeconds DeltaSeconds)
  (CallFunction|DamageCharacter (LocalVariables|GetLocalCharacter) (* (Variables|Settings|TickDamage|GetTickDamagePerSecond) (LocalVariables|GetLocalDeltaSeconds)) (Variables|Settings|TickDamage|GetTickDamageType) (Variables|Settings|TickDamage|GetTickCriticalHit) (Variables|Settings|TickDamage|GetTickBreakBlock) (Variables|Settings|TickDamage|GetTickInterruptAnimation) (Variables|Settings|TickDamage|GetTickShowPlayerReactionEffects))
  (return true))

(fn DamageCharacter
  (params (Character :type Character%20Object%20Reference) (Damage :type Float%20%28single-precision%29) (DamageType :type Damage%20Type%20Class%20Reference) (CriticalHit :type Boolean) (BreakBlock :type Boolean) (InterruptAnimation :type Boolean) (ShowPlayerReactionEffects :type Boolean))
  ;[1 1 1] Apply damage to character.
  (if (> Damage 0.0)
    (CallFunction|ApplyAdvancedPointDamage :DamagedActor Character :DamageData (Utilities|Struct|MakeSTR_DamageData Damage DamageType CriticalHit BreakBlock InterruptAnimation ShowPlayerReactionEffects) :DamageCauser self)
    (return true)))

(fn SetActivatedState
  (params (NewActivatedState :type Boolean))
  ;[1 1 1] Set activated state.
  (bind _output_get (Variables|State|SetIsActivated NewActivatedState))
  (Actor|Tick|SetActorTickEnabled _output_get)
  (return true))