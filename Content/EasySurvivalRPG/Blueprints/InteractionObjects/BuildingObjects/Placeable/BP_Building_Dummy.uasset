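; Placeable training dummy building object that plays a hit animation when damaged.
; It supplies four floor checkers and a build collision for placement checks, and can destroy that collision component.
; Its static Mesh shows until built, then the SkeletalMesh replaces it.
; Damage calls the parent handler, then multicasts the hit animation if the dummy is damageable and has durability left.
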(event Custom|UpdateBuildedMeshes
  (bind _built (Variables|Default|GetBuilt))
  ;[1 1 1] Begin play. Update meshes.
  (Development|SetHiddeninGame (Variables|Character|GetMesh) _built true)
  (Development|SetHiddeninGame (Variables|Default|GetSkeletalMesh) (not _built) true))

(event Custom|PlayHit%20%28Multicast%29
  ;[1 1 1] Interactions when takes damage.
  (Components|Animation|PlayAnimation (Variables|Default|GetSkeletalMesh) "/Game/EasySurvivalRPG/Meshes/SKMeshes/A_Dummy_Hit.A_Dummy_Hit" false))

(event EventBeginPlay
  ;[1 1 1] Begin play. Update meshes.
  (|CallParentFunction)
  (CallFunction|UpdateBuildedMeshes))

(event EventDamageTaken
  (params (DamageData :type STR%20Damage%20Data%20Structure%20%28by%20ref%29) (InstigatedBy :type Controller%20Object%20Reference) (DamageCauser :type Actor%20Object%20Reference) (HitInfo :type Hit%20Result%20Structure))
  ;[1 1 1] Interactions when takes damage.
  (|CallParentFunction DamageData InstigatedBy DamageCauser HitInfo)
  (if (and (Variables|Default|GetbCanBeDamaged) (> (Variables|Default|GetDurability) 0.0))
    (CallFunction|PlayHit(Multicast))))

(event EventSetFloorCheckers
  ;[1 1 1] Overridden Events.
  (Variables|Default|SetFloorCheckers (Utilities|Array|MakeArray (Variables|Default|GetFloorChecker1) (Variables|Default|GetFloorChecker2) (Variables|Default|GetFloorChecker3) (Variables|Default|GetFloorChecker4))))

(event EventDestroyBuildComponents
  ;[1 1 1] Overridden Events.
  (Components|DestroyComponent (Variables|Default|GetBuildCollision)))

(fn ConstructionScript
  (|CallParentFunction))

(fn CheckBuildCollisions
  (params (Actor :type Actor%20Object%20Reference))
  (return (CallFunction|CheckActorCollisions Actor (Variables|Default|GetBuildCollision))))