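; Medium crop plot building piece for the survival game's farming system, providing two sockets for plants.
; It overrides socket creation to cache the world transforms of its two PlantSocket components.
; Socket lookups return a cached transform by clamped index.
; Occupancy checks report whether a given building object's location matches either socket within a small tolerance.
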(event EventCreateSocketTransforms
  ;[1 1 1] Overrided Events.
  (Variables|Default|SetPlantSocketTransforms (Utilities|Array|MakeArray (Transformation|GetWorldTransform (Variables|Default|GetPlantSocket1)) (Transformation|GetWorldTransform (Variables|Default|GetPlantSocket2)))))

(fn ConstructionScript
  (|CallParentFunction))

(fn GetSocketTransform
  (params (SocketName :type Name :default "None") (Index :type Integer))
  (switch name SocketName
    (:Plant
      (return (Utilities|Array|Get(acopy) (Variables|Default|GetPlantSocketTransforms) (Math|Integer|Clamp(Integer) Index 0 1))))))

(fn BuildingObjectinSocket
  (params (BuildingObject :type BP%20Building%20Building%20Object%20Object%20Reference))
  (for _array_element (Variables|Default|GetPlantSocketTransforms)
    (if (Math|Vector|Equal(Vector) (.Location (Math|Transform|BreakTransform _array_element)) (Transformation|GetActorLocation BuildingObject) 1.0)
      (return (Math|Vector|Equal(Vector) (.Location (Math|Transform|BreakTransform _array_element)) (Transformation|GetActorLocation BuildingObject) 1.0))))
  (return false))