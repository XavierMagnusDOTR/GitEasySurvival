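; Base Blueprint for placeable table decorations in the survival RPG building system, specializing a parent building object.
; It overrides SetFloorCheckers to register four floor checker components for the floor check.
; CheckBuildCollisions tests a target actor against the BuildCollision component, returning true when that actor does not block placement.
; The construction script only calls the parent's.
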(event EventSetFloorCheckers
  ;[1 1 1] Overriden function for floor checking.
  (Variables|Default|SetFloorCheckers (Utilities|Array|MakeArray (Variables|Default|GetFloorChecker1) (Variables|Default|GetFloorChecker2) (Variables|Default|GetFloorChecker3) (Variables|Default|GetFloorChecker4))))

(fn ConstructionScript
  (|CallParentFunction))

(fn CheckBuildCollisions
  (params (Actor :type Actor%20Object%20Reference))
  ;[1 1 1] Returns true if target actor does not block build collisions.
  (return (CallFunction|CheckActorCollisions Actor (Variables|Default|GetBuildCollision))))