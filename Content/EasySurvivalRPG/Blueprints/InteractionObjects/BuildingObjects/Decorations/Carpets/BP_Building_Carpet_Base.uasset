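; Base Blueprint for placeable carpet decorations in the survival game's building system, specializing inherited placement checks.
; It registers four floor checker components for floor validation and reports the actor's own Z location as floor height.
; Its build collision check lets carpets overlap any non-carpet actor, rejecting only other carpets that overlap its BuildCollision component.
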(event EventSetFloorCheckers
  ;[1 1 1] Overriden function for floor checking.
  (Variables|Default|SetFloorCheckers (Utilities|Array|MakeArray (Variables|Default|GetFloorChecker1) (Variables|Default|GetFloorChecker2) (Variables|Default|GetFloorChecker3) (Variables|Default|GetFloorChecker4))))

(fn ConstructionScript
  (|CallParentFunction))

(fn CheckBuildCollisions
  (params (Actor :type Actor%20Object%20Reference))
  ;[1 1 1] Returns true if target actor does not block build collisions.
  (Utilities|Casting|CastToBP_Building_Carpet_Base Actor
    (:then
      (return (not (Collision|IsOverlappingActor (Variables|Default|GetBuildCollision) Actor :!class /Script/Engine.PrimitiveComponent))))
    (:CastFailed
      (return true))))

(fn GetFloorZ
  (return (.z (Transformation|GetActorLocation))))