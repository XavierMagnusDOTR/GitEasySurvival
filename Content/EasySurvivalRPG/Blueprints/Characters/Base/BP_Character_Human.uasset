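; Base human AI character for the survival RPG, armed and dressed from item data.
; Construction script previews custom weapon and equipment meshes in editor; on init the authority grants those items, or randomized sets if uncustomized.
; Combat events drive attacks, bow charging and server-side shooting with recoil, durability loss, item abilities and timed fire rate.
; Weapon stance selects melee, ranged or bow behavior tree unless overridden; death adds loot.
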(event EventMakeDeathLoot
  (bind _loothandle (Variables|Default|GetLootHandle))
  ;[1 1 1] Death loot.
  (if (CallFunction|HandleIsValid _loothandle)
    (Default|TryAddItems (Variables|Default|GetInventoryContainer) (CallFunction|MakeLootItems _loothandle)))
  (|CallParentFunction))

(event EventEquipmentChanged
  (params (EquipmentSlot :type E_EquipmentSlot%20Enum :default "NewEnumerator0") (Item :type STR%20Item%20Data%20Structure))
  ;[1 1 1] Update character initialy states for equipment.
  (|CallParentFunction EquipmentSlot Item)
  (Utilities|FlowControl|DoOnce false
    (:Completed
      (CallFunction|ChangeHealth 1.0 true))))

(event EventTryAttackBPI
  ;[1 1 1] Combat events.
  (CallFunction|TryAttack))

(event EventTryChargeBPI
  ;[1 1 1] Combat events.
  (CallFunction|TryChargeInteraction))

(event EventTryShootBPI
  ;[1 1 1] Combat events.
  (CallFunction|TryStartShooting))

(event EventTryReleaseChargeBPI
  ;[1 1 1] Combat events.
  (CallFunction|SetChargingMode false))

(fn ConstructionScript
  (|CallParentFunction)
  (if (CallFunction|RuninEditor)
    (Customisation|UpdatePreviewWeapon)
    (Customisation|UpdatePreviewHeadMesh)
    (Customisation|UpdatePreviewBodyMesh)
    (Customisation|UpdatePreviewPantsMesh)
    (Customisation|UpdatePreviewHandsMesh)
    (Customisation|UpdatePreviewFeetMesh)))

(fn TryShoot
  (params (Anim :type STR%20Anim%20Montage%20Play%20Data%20Structure))
  ;[1 1 1] Try shoot with selected weapon.
  (LocalVariables|SetLocalAnim Anim)
  (bind _output_get (LocalVariables|SetLocalItem (Default|GetSelectedItem (Variables|Default|GetHotbarContainer))))
  (bind _success (Default|CheckAbilityConditions (Variables|Default|GetAbilitySystemComponent) (CallFunction|GetItemAbilityHandle _output_get) (CallFunction|GetItemUseAbility _output_get)))
  (if _success
    (CallFunction|PlayAnimation(Multicast) (LocalVariables|GetLocalAnim))
    (Class|BPIUsableItem|PlayShootAnimationBPI(Message) (Variables|Default|GetUsableItemActor) (Variables|Default|GetShouldAiming))
    (return true)
    (else
      (return false))))

(fn TryChargeInteraction
  ;[1 1 1] Try charge interaction and play bow start animation.
  (LocalVariables|SetLocalItem (Default|GetSelectedItem (Variables|Default|GetHotbarContainer)))
  (if (CallFunction|IsCanInteract)
    (CallFunction|PlayAnimation(Multicast) (Variables|Default|GetBowStartShootAnim))
    (Class|BPIUsableItem|PlayChargeAnimationBPI(Message) (Variables|Default|GetUsableItemActor))
    (CallFunction|SetChargingMode true)
    (return true)
    (else
      (return false))))

(fn Shoot
  (params (AimedShoot :type Boolean))
  (bind _attributescomponent (Variables|Default|GetAttributesComponent))
  (bind _attributescomponent_2 (Variables|Default|GetAttributesComponent))
  (bind _value (Default|GetAttributeValue _attributescomponent_2 "(TagName=\"EasyRPG.Attributes.Weapon.ShootingRate\")"))
  ;[1 1 1] Shoot with current selected weapon.
  (Networking|SwitchHasAuthority
    (:Authority
      (bind _output_get (LocalVariables|SetLocalItem (Default|GetSelectedItem (Variables|Default|GetHotbarContainer))))
      (CallFunction|PlaySoundatLocation(Multicast) (CallFunction|GetItemSound _output_get "Shoot") (Transformation|GetActorLocation))
      (Class|BPIPlayer|PlayShotReactionBPI(Message) (Pawn|GetController) (Default|GetAttributeValue _attributescomponent "(TagName=\"EasyRPG.Attributes.Weapon.ShootingRecoilScale\")") (Default|GetAttributeValue _attributescomponent "(TagName=\"EasyRPG.Attributes.Weapon.ShootingRecoilOffset\")"))
      (CallFunction|SpawnShootEffects)
      (CallFunction|ItemUsedServer)
      (Variables|Default|SetCanContinueShooting (CallFunction|ItemIsContinuable (LocalVariables|GetLocalItem)))
      (CallFunction|TrytoChangeItemDurability (Variables|Default|GetInteractionItemContainer) (Variables|Default|GetInteractionItemSlot) -1.0)
      (bind _output_get_2 (LocalVariables|SetLocalShootingRate (select (> _value 0.0) _value 6e+01)))
      (Variables|Default|SetBlockContinueShooting true)
      (Utilities|Time|SetTimerbyEvent (EventDispatchers|CreateEvent :!event ResetShootingBlock) (/ 6e+01 _output_get_2))
      (return true))
    (:Remote
      (return false))))

(fn ItemUsedServer
  ;[1 1 1] Use ability of the selected item.
  (bind _output_get (LocalVariables|SetLocalItem (Default|GetSelectedItem (Variables|Default|GetHotbarContainer))))
  (if (CallFunction|ItemIsConsumable _output_get)
    (Class|BPIPlayer|TrytoConsumeItemBPI(Message) (Pawn|GetController) (Variables|Default|GetInteractionItemContainer) (Variables|Default|GetInteractionItemSlot)))
  (Default|TrytoUseAbility (Variables|Default|GetAbilitySystemComponent) (CallFunction|GetItemAbilityHandle (LocalVariables|GetLocalItem)) (CallFunction|GetItemUseAbility (LocalVariables|GetLocalItem)))
  (return true))

(fn UpdateBehaviorTree
  (bind _overriddenbehaviortree (Variables|Default|GetOverriddenBehaviorTree))
  (bind _meleebehavior (Variables|Settings|AI|GetMeleeBehavior))
  (bind _rangedbehavior (Variables|Settings|AI|GetRangedBehavior))
  ;[1 1 1] Update behavior tree depending on stance.
  (bind _returnvalue (AI|RunBehaviorTree (AI|GetAIController self) (select (Utilities|IsValid _overriddenbehaviortree) _overriddenbehaviortree (Utilities|Select :Index (Variables|Default|GetStance) :NewEnumerator0 _meleebehavior :NewEnumerator1 _meleebehavior :NewEnumerator2 _meleebehavior :NewEnumerator6 0 :NewEnumerator7 0 :NewEnumerator8 0 :NewEnumerator9 0 :NewEnumerator10 _meleebehavior :NewEnumerator11 _meleebehavior :NewEnumerator12 _meleebehavior :NewEnumerator16 _meleebehavior :NewEnumerator13 _rangedbehavior :NewEnumerator14 _rangedbehavior :NewEnumerator15 _rangedbehavior :NewEnumerator17 _rangedbehavior :NewEnumerator18 _rangedbehavior :NewEnumerator19 0 :NewEnumerator20 _rangedbehavior :NewEnumerator21 _rangedbehavior :NewEnumerator22 (Variables|Settings|AI|GetBowBehavior) :NewEnumerator23 0 :NewEnumerator24 0))))
  (return _returnvalue))

(fn RandomizeWeapon
  (bind _randomweapon (Variables|Settings|Customisation|GetRandomWeapon))
  (bind _item (CallFunction|MakeRandomLootItem _randomweapon))
  ;[1 1 1] Set random weapon from item list.
  (if (CallFunction|HandleIsValid _randomweapon)
    (bind _output_get (LocalVariables|SetLocalItem _item))
    (if (CallFunction|RuninEditor)
      (Variables|Settings|Customisation|SetCustomWeaponItem _item)
      (Customisation|UpdatePreviewWeapon)
      (else
        (Default|TryAddItems (Variables|Default|GetHotbarContainer) (Utilities|Array|MakeArray _output_get))))))

(fn RandomizeEquipment
  (bind _randomequipmentsets (Variables|Settings|Customisation|GetRandomEquipmentSets))
  ;[1 1 1] Set equipment items from random equipment set and update character equipment.
  (bind _output_get (LocalVariables|SetLocalEquipmentSet (Utilities|Array|Get(acopy) _randomequipmentsets (Math|Random|RandomIntegerinRange 0 (Utilities|Array|LastIndex _randomequipmentsets)))))
  (if (CallFunction|RuninEditor)
    (Variables|Settings|Customisation|SetCustomHeadItem "")
    (Variables|Settings|Customisation|SetCustomBodyItem "")
    (Variables|Settings|Customisation|SetCustomPantsItem "")
    (Variables|Settings|Customisation|SetCustomHandsItem "")
    (Variables|Settings|Customisation|SetCustomFeetItem "")
    (for _array_element (CallFunction|MakeLootItems _output_get)
      (LocalVariables|SetLocalItem _array_element)
      (if (.Result (CallFunction|ItemIsEquipment (CallFunction|MakeItembyHandle (.ItemHandle (Utilities|Struct|BreakSTR_Item _array_element)) (.Amount (Utilities|Struct|BreakSTR_Item _array_element)) (.Charges (Utilities|Struct|BreakSTR_Item _array_element)) (.Durability (Utilities|Struct|BreakSTR_Item _array_element)) (.Decay (Utilities|Struct|BreakSTR_Item _array_element)))))
        (switch Utilities|FlowControl|Switch|SwitchonE_EquipmentSlot (.EquipmentSlot (CallFunction|ItemIsEquipment (CallFunction|MakeItembyHandle (.ItemHandle (Utilities|Struct|BreakSTR_Item _array_element)) (.Amount (Utilities|Struct|BreakSTR_Item _array_element)) (.Charges (Utilities|Struct|BreakSTR_Item _array_element)) (.Durability (Utilities|Struct|BreakSTR_Item _array_element)) (.Decay (Utilities|Struct|BreakSTR_Item _array_element)))))
          (:NewEnumerator0
            (Variables|Settings|Customisation|SetCustomHeadItem (LocalVariables|GetLocalItem)))
          (:NewEnumerator1
            (Variables|Settings|Customisation|SetCustomBodyItem (LocalVariables|GetLocalItem)))
          (:NewEnumerator2
            (Variables|Settings|Customisation|SetCustomPantsItem (LocalVariables|GetLocalItem)))
          (:NewEnumerator3
            (Variables|Settings|Customisation|SetCustomHandsItem (LocalVariables|GetLocalItem)))
          (:NewEnumerator4
            (Variables|Settings|Customisation|SetCustomFeetItem (LocalVariables|GetLocalItem))))))
    (Customisation|UpdatePreviewHeadMesh)
    (Customisation|UpdatePreviewBodyMesh)
    (Customisation|UpdatePreviewPantsMesh)
    (Customisation|UpdatePreviewHandsMesh)
    (Customisation|UpdatePreviewFeetMesh)
    (else
      (Default|TryAddItems (Variables|Default|GetEquipmentContainer) (CallFunction|MakeLootItems _output_get)))))

(fn InitCharacter
  ;[1 1 1] Init character and update equipment equipment.
  (|CallParentFunction)
  (Components|DestroyComponent (Variables|Default|GetPreviewWeaponStaticMesh))
  (Networking|SwitchHasAuthority
    (:Authority
      (if (Variables|Settings|Customisation|GetCustomisationOn)
        (Default|TryAddItems (Variables|Default|GetHotbarContainer) (Utilities|Array|MakeArray (Variables|Settings|Customisation|GetCustomWeaponItem)))
        (Default|TryAddItems (Variables|Default|GetEquipmentContainer) (Utilities|Array|MakeArray (Variables|Settings|Customisation|GetCustomHeadItem) (Variables|Settings|Customisation|GetCustomBodyItem) (Variables|Settings|Customisation|GetCustomPantsItem) (Variables|Settings|Customisation|GetCustomHandsItem) (Variables|Settings|Customisation|GetCustomFeetItem)))
        (else
          (Settings|RandomizeEquipment)
          (Settings|RandomizeWeapon)))
      (return true))))

(fn UpdatePreviewWeapon
  (bind _customweaponitem (Variables|Settings|Customisation|GetCustomWeaponItem))
  (bind _previewweaponstaticmesh (Variables|Default|GetPreviewWeaponStaticMesh))
  (bind _previewweaponskeletalmesh (Variables|Default|GetPreviewWeaponSkeletalMesh))
  (bind (_itemhandle _amount _charges _durability _decay) (Utilities|Struct|BreakSTR_Item _customweaponitem))
  ;[1 1 1] Update preview weapon meshes of the character.
  (if (CallFunction|ItemHandleIsValid _itemhandle)
    (bind _output_get (LocalVariables|SetLocalItem (CallFunction|MakeItembyHandle _itemhandle _amount _charges _durability _decay)))
    (if (and (.IsWeapon (CallFunction|ItemIsWeapon _output_get)) (CallFunction|ItemIsUsable _output_get))
      (if (.Found (CallFunction|GetItemUsableData _output_get))
        (Rendering|SetVisibility (Variables|Default|GetPreviewWeaponStaticMesh) true false)
        (Components|StaticMesh|SetStaticMesh _previewweaponstaticmesh (.StaticMesh (Utilities|Struct|BreakSTR_UsableItemData (.UsableItemData (CallFunction|GetItemUsableData _output_get)))))
        (Transformation|AttachComponentToComponent _previewweaponstaticmesh (Variables|Character|GetMesh) (.SocketName (Utilities|Struct|BreakSTR_UsableItemData (.UsableItemData (CallFunction|GetItemUsableData _output_get)))) "SnapToTarget" "SnapToTarget" "SnapToTarget" true)
        (Class|SkinnedMeshComponent|SetSkeletalMesh _previewweaponskeletalmesh (.SkeletalMesh (Utilities|Struct|BreakSTR_UsableItemData (.UsableItemData (CallFunction|GetItemUsableData _output_get)))) true)
        (Transformation|AttachComponentToComponent _previewweaponskeletalmesh (Variables|Character|GetMesh) (.SocketName (Utilities|Struct|BreakSTR_UsableItemData (.UsableItemData (CallFunction|GetItemUsableData _output_get)))) "SnapToTarget" "SnapToTarget" "SnapToTarget" true)
        (Variables|Settings|Customisation|SetCustomisationOn true)
        (else
          (Development|PrintString "Wrong weapon item!" true true "(R=1.000000,G=0.000000,B=0.000000,A=1.000000)" 5.0 :!label _label)
          (Rendering|SetVisibility (Variables|Default|GetPreviewWeaponStaticMesh) false false :!label _label_2)))
      (else
        (goto _label)))
    (else
      (goto _label_2))))

(fn UpdatePreviewHeadMesh
  (bind _customheaditem (Variables|Settings|Customisation|GetCustomHeadItem))
  (bind (_itemhandle _amount _charges _durability _decay) (Utilities|Struct|BreakSTR_Item _customheaditem))
  ;[1 1 1] Update custom preview head mesh of the character.
  (if (CallFunction|ItemHandleIsValid _itemhandle)
    (bind _output_get (LocalVariables|SetLocalItem (CallFunction|MakeItembyHandle _itemhandle _amount _charges _durability _decay)))
    (if (and (.Result (CallFunction|ItemIsEquipment _output_get)) (Utilities|Enum|Equal(Enum) (.EquipmentSlot (CallFunction|ItemIsEquipment _output_get)) "NewEnumerator0"))
      (Variables|Default|SetEquipedHeadMesh (CallFunction|GetItemSkeletalMesh _output_get (Variables|Default|GetEquipmentCharacterID)))
      (Variables|Settings|Customisation|SetCustomisationOn true)
      (else
        (Development|PrintString "Wrong head item!" true true "(R=1.000000,G=0.000000,B=0.000000,A=1.000000)" 5.0)
        (Variables|Default|SetEquipedHeadMesh 0 :!label _label)))
    (else
      (goto _label))))

(fn UpdatePreviewBodyMesh
  (bind _custombodyitem (Variables|Settings|Customisation|GetCustomBodyItem))
  (bind (_itemhandle _amount _charges _durability _decay) (Utilities|Struct|BreakSTR_Item _custombodyitem))
  ;[1 1 1] Update custom preview body mesh of the character.
  (if (CallFunction|ItemHandleIsValid _itemhandle)
    (bind _output_get (LocalVariables|SetLocalItem (CallFunction|MakeItembyHandle _itemhandle _amount _charges _durability _decay)))
    (if (and (.Result (CallFunction|ItemIsEquipment _output_get)) (Utilities|Enum|Equal(Enum) (.EquipmentSlot (CallFunction|ItemIsEquipment _output_get)) "NewEnumerator1"))
      (Variables|Default|SetEquipedBodyMesh (CallFunction|GetItemSkeletalMesh _output_get (Variables|Default|GetEquipmentCharacterID)))
      (Variables|Settings|Customisation|SetCustomisationOn true)
      (else
        (Development|PrintString "Wrong body item!" true true "(R=1.000000,G=0.000000,B=0.000000,A=1.000000)" 5.0)
        (Variables|Default|SetEquipedBodyMesh 0 :!label _label)))
    (else
      (goto _label))))

(fn UpdatePreviewPantsMesh
  (bind _custompantsitem (Variables|Settings|Customisation|GetCustomPantsItem))
  (bind (_itemhandle _amount _charges _durability _decay) (Utilities|Struct|BreakSTR_Item _custompantsitem))
  ;[1 1 1] Update custom preview pants mesh of the character.
  (if (CallFunction|ItemHandleIsValid _itemhandle)
    (bind _output_get (LocalVariables|SetLocalItem (CallFunction|MakeItembyHandle _itemhandle _amount _charges _durability _decay)))
    (if (and (.Result (CallFunction|ItemIsEquipment _output_get)) (Utilities|Enum|Equal(Enum) (.EquipmentSlot (CallFunction|ItemIsEquipment _output_get)) "NewEnumerator2"))
      (Variables|Default|SetEquipedPantsMesh (CallFunction|GetItemSkeletalMesh _output_get (Variables|Default|GetEquipmentCharacterID)))
      (Variables|Settings|Customisation|SetCustomisationOn true)
      (else
        (Development|PrintString "Wrong pants item!" true true "(R=1.000000,G=0.000000,B=0.000000,A=1.000000)" 5.0)
        (Variables|Default|SetEquipedPantsMesh 0 :!label _label)))
    (else
      (goto _label))))

(fn UpdatePreviewHandsMesh
  (bind _customhandsitem (Variables|Settings|Customisation|GetCustomHandsItem))
  (bind (_itemhandle _amount _charges _durability _decay) (Utilities|Struct|BreakSTR_Item _customhandsitem))
  ;[1 1 1] Update custom preview hands mesh of the character.
  (if (CallFunction|ItemHandleIsValid _itemhandle)
    (bind _output_get (LocalVariables|SetLocalItem (CallFunction|MakeItembyHandle _itemhandle _amount _charges _durability _decay)))
    (if (and (.Result (CallFunction|ItemIsEquipment _output_get)) (Utilities|Enum|Equal(Enum) (.EquipmentSlot (CallFunction|ItemIsEquipment _output_get)) "NewEnumerator3"))
      (Variables|Default|SetEquipedHandsMesh (CallFunction|GetItemSkeletalMesh _output_get (Variables|Default|GetEquipmentCharacterID)))
      (Variables|Settings|Customisation|SetCustomisationOn true)
      (else
        (Development|PrintString "Wrong hands item!" true true "(R=1.000000,G=0.000000,B=0.000000,A=1.000000)" 5.0)
        (Variables|Default|SetEquipedHandsMesh 0 :!label _label)))
    (else
      (goto _label))))

(fn UpdatePreviewFeetMesh
  (bind _customfeetitem (Variables|Settings|Customisation|GetCustomFeetItem))
  (bind (_itemhandle _amount _charges _durability _decay) (Utilities|Struct|BreakSTR_Item _customfeetitem))
  ;[1 1 1] Update custom preview feet mesh of the character.
  (if (CallFunction|ItemHandleIsValid _itemhandle)
    (bind _output_get (LocalVariables|SetLocalItem (CallFunction|MakeItembyHandle _itemhandle _amount _charges _durability _decay)))
    (if (and (.Result (CallFunction|ItemIsEquipment _output_get)) (Utilities|Enum|Equal(Enum) (.EquipmentSlot (CallFunction|ItemIsEquipment _output_get)) "NewEnumerator4"))
      (Variables|Default|SetEquipedFeetMesh (CallFunction|GetItemSkeletalMesh _output_get (Variables|Default|GetEquipmentCharacterID)))
      (Variables|Settings|Customisation|SetCustomisationOn true)
      (else
        (Development|PrintString "Wrong feet item!" true true "(R=1.000000,G=0.000000,B=0.000000,A=1.000000)" 5.0)
        (Variables|Default|SetEquipedFeetMesh 0 :!label _label)))
    (else
      (goto _label))))

(fn ClearCustomisation
  (Variables|Settings|Customisation|SetCustomWeaponItem "")
  (Customisation|UpdatePreviewWeapon)
  (Variables|Settings|Customisation|SetCustomHeadItem "")
  (Variables|Settings|Customisation|SetCustomBodyItem "")
  (Variables|Settings|Customisation|SetCustomPantsItem "")
  (Variables|Settings|Customisation|SetCustomHandsItem "")
  (Variables|Settings|Customisation|SetCustomFeetItem "")
  (Customisation|UpdatePreviewHeadMesh)
  (Customisation|UpdatePreviewBodyMesh)
  (Customisation|UpdatePreviewPantsMesh)
  (Customisation|UpdatePreviewHandsMesh)
  (Customisation|UpdatePreviewFeetMesh)
  (Variables|Settings|Customisation|SetCustomisationOn false))

(fn RefreshInitialyStates
  ;[1 1 1] Refresh initialy states of the character to maximum values.
)