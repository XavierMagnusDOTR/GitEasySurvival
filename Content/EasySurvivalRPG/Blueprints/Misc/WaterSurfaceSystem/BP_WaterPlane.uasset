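; BP_WaterPlane is a water surface actor in the Water Surface System that builds a tiled water plane from mesh instances.
; Its Construction Script applies the water material, then rebuilds a PlaneSize grid of WaterPlane instances spaced by the mesh's local bounds.
; It offsets the component by half the grid span to center the tiles on the actor.
; The caustic decal component is destroyed when the Caustic flag is off.
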(fn ConstructionScript
  ;[1 1 1] Construct water plane.
  (Rendering|Material|SetMaterial (Variables|Default|GetWaterPlane) 0 (Variables|WaterPlane|GetWaterMaterial))
  (CallFunction|CreateWaterInstances))

(fn CreateWaterInstances
  (bind _waterplane (Variables|Default|GetWaterPlane))
  (bind _planesize (Variables|WaterPlane|GetPlaneSize))
  (bind _planesize_2 (Variables|WaterPlane|GetPlaneSize))
  (bind _waterplane_2 (Variables|Default|GetWaterPlane))
  (bind _max (Components|StaticMesh|GetLocalBounds _waterplane_2))
  (bind _max_2 (Components|StaticMesh|GetLocalBounds _waterplane))
  (bind (_x _y) (Math|Vector|BreakVector _max))
  (bind (_x_2 _y_2) (Math|Vector|BreakVector _max_2))
  ;[1 1 1] Create water plane instances.
  (Components|InstancedStaticMesh|ClearInstances (Variables|Default|GetWaterPlane))
  (for _index (range 0 (- (Math|Float|Floor (.x _planesize_2)) 1))
    (LocalVariables|SetLocalX _index)
    (for _index_2 (range 0 (- (Math|Float|Floor (.y _planesize_2)) 1))
      (LocalVariables|SetLocalY _index_2)
      (Components|InstancedStaticMesh|AddInstance (Variables|Default|GetWaterPlane) (Math|Transform|MakeTransform (Math|Vector|MakeVector (* (LocalVariables|GetLocalX) (* _x 2.0)) (* (LocalVariables|GetLocalY) (* _y 2.0)) 0.0)))))
  (Transformation|SetRelativeLocation _waterplane (Math|Vector|MakeVector (- 0.0 (* (- (Math|Float|Floor (.x _planesize)) 1) _x_2)) (- 0.0 (* (- (Math|Float|Floor (.y _planesize)) 1) _y_2)) 0.0) false false)
  (if (not (Variables|WaterPlane|GetCaustic))
    (Components|DestroyComponent (Variables|Default|GetCausticDecal))))