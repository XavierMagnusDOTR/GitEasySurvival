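; Deprecated actor, superseded by BP_SplineMovedActor_Mesh, that moves spawned static meshes along a spline at a set speed.
; Spawns come from BeginPlay, random-delay timers or Character trigger overlaps, gated by max count and chance.
; Tick advances each mesh's time in parallel arrays, then destroys it or resets its time at the end.
; Construction derives spline duration from length and speed, and can snap the last point onto the first.
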(event OnActorBeginOverlap(Trigger)
  (params (OverlappedActor :type Actor%20Object%20Reference) (OtherActor :type Actor%20Object%20Reference))
  ;[1 0 0] NOTE: Use BP_SplineMovedActor_Mesh instead this blueprint!!!
  (Utilities|Casting|CastToCharacter OtherActor)
  (CallFunction|SpawnandMovetoSpline))

(event Custom|SpawnTimer
  ;[1 0 0] NOTE: Use BP_SplineMovedActor_Mesh instead this blueprint!!!
  (CallFunction|SpawnandMovetoSpline)
  (if (< (Utilities|Array|Length (Variables|Default|GetMovedMeshes)) (Variables|Spawn|GetMaxCount))
    (Utilities|Time|SetTimerbyEvent (EventDispatchers|CreateEvent :!event Custom|SpawnTimer) (Math|Random|RandomFloatinRange (Variables|Spawn|GetMinSpawnDelay) (Variables|Spawn|GetMaxSpawnDelay)))))

(event EventTick
  (params (DeltaSeconds :type Float%20%28single-precision%29))
  (bind _movedtimes (Variables|Default|GetMovedTimes))
  (bind _spline (Variables|Default|GetSpline))
  (bind _duration (Variables|/Script/Engine.SplineComponent|GetDuration _spline))
  ;[1 0 0] NOTE: Use BP_SplineMovedActor_Mesh instead this blueprint!!!
  (for (_array_element _array_index) (Variables|Default|GetMovedMeshes)
    (Utilities|Array|SetArrayElem _movedtimes _array_index (Math|Float|Clamp(Float) (+ (Utilities|Array|Get(acopy) _movedtimes _array_index) DeltaSeconds) 0.0 _duration))
    (CallFunction|UpdateMeshPosition _array_element (Utilities|Array|Get(acopy) _movedtimes _array_index))
    (if (== (Math|Float|Clamp(Float) (+ (Utilities|Array|Get(acopy) _movedtimes _array_index) DeltaSeconds) 0.0 _duration) _duration)
      (if (Variables|Spawn|GetDestroyWhenFinish)
        (Components|DestroyComponent _array_element)
        (Utilities|Array|RemoveIndex (Variables|Default|GetMovedMeshes) _array_index)
        (Utilities|Array|RemoveIndex (Variables|Default|GetMovedTimes) _array_index)
        (Utilities|Time|SetTimerbyEvent (EventDispatchers|CreateEvent :!event Custom|SpawnTimer) (Math|Random|RandomFloatinRange (Variables|Spawn|GetMinSpawnDelay) (Variables|Spawn|GetMaxSpawnDelay)))
        (else
          (Utilities|Array|SetArrayElem (Variables|Default|GetMovedTimes) _array_index 0.0))))))

(event EventBeginPlay
  ;[1 0 0] NOTE: Use BP_SplineMovedActor_Mesh instead this blueprint!!!
  (Components|DestroyComponent (Variables|Default|GetMesh))
  (if (Variables|Spawn|GetSpawnOnBeginPlay)
    (CallFunction|SpawnandMovetoSpline))
  (if (Variables|Spawn|GetSpawnOnTimer)
    (Utilities|Time|SetTimerbyEvent (EventDispatchers|CreateEvent :!event Custom|SpawnTimer) (Math|Random|RandomFloatinRange (Variables|Spawn|GetMinSpawnDelay) (Variables|Spawn|GetMaxSpawnDelay)))))

(fn ConstructionScript
  (bind _spline (Variables|Default|GetSpline))
  (Variables|/Script/Engine.SplineComponent|SetDuration _spline (/ (Spline|GetSplineLength _spline) (Variables|Spawn|GetMovementSpeed)))
  (Components|StaticMesh|SetStaticMesh (Variables|Default|GetMesh) (Variables|Spawn|GetStaticMesh))
  (CallFunction|CorrectCycledSpline))

(fn SpawnandMovetoSpline
  (bind _maxcount (Variables|Spawn|GetMaxCount))
  (if (and (or (== _maxcount 0) (< (Utilities|Array|Length (Variables|Default|GetMovedMeshes)) _maxcount)) (<= (Math|Random|RandomFloat) (Variables|Spawn|GetTriggerChance)))
    (bind _returnvalue (AddComponent|AddStaticMeshComponent false))
    (bind _output_get (LocalVariables|SetLocalMesh _returnvalue))
    (Components|StaticMesh|SetStaticMesh _output_get (Variables|Spawn|GetStaticMesh))
    (CallFunction|UpdateMeshPosition _output_get 0.0)
    (Utilities|Array|Add (Variables|Default|GetMovedMeshes) _output_get)
    (Utilities|Array|Add (Variables|Default|GetMovedTimes) 0.0)))

(fn UpdateMeshPosition
  (params (Mesh :type Mesh%20Component%20Object%20Reference) (Time :type Float%20%28single-precision%29))
  (Transformation|SetRelativeTransform Mesh (Spline|GetTransformatTime (Variables|Default|GetSpline) Time "Local" false false) false false)
  (Transformation|AddRelativeRotation Mesh "0,90.000000, 0" false false))

(fn RefreshPoints
  (bind _spline (Variables|Default|GetSpline))
  (bind _spline_2 (Variables|Default|GetSpline))
  (bind _spline_3 (Variables|Default|GetSpline))
  (bind _returnvalue (Spline|GetNumberOfSplinePoints _spline))
  (bind _returnvalue_2 (- _returnvalue 1))
  (CallFunction|CorrectCycledSpline)
  (LocalVariables|SetLocalPoints _returnvalue)
  (LocalVariables|SetLocalDif (/ (Spline|GetSplineLength _spline) (Math|Conversions|ToFloat(Integer) _returnvalue_2)))
  (for _index (range 0 _returnvalue_2)
    (Utilities|Array|Add (LocalVariables|GetLocalSplinePoints) (Utilities|Struct|MakeSplinePoint (Math|Conversions|ToFloat(Integer) _index) (Spline|GetLocationatDistanceAlongSpline _spline_2 (* (LocalVariables|GetLocalDif) (Math|Conversions|ToFloat(Integer) _index)) "Local") "0.000000,0.000000,0.000000" "0.000000,0.000000,0.000000" (Spline|GetRotationatDistanceAlongSpline _spline_2 (* (LocalVariables|GetLocalDif) (Math|Conversions|ToFloat(Integer) _index)) "Local"))))
  (Spline|ClearSplinePoints _spline_3 false)
  (Class|SplineComponent|AddPoints _spline_3 (LocalVariables|GetLocalSplinePoints) true))

(fn CorrectCycledSpline
  (bind _spline (Variables|Default|GetSpline))
  (bind _returnvalue (Spline|GetNumberOfSplinePoints _spline))
  (if (and (Variables|Spawn|GetCycledSpline) (> _returnvalue 2))
    (Spline|SetLocationatSplinePoint _spline (- _returnvalue 1) (Spline|GetLocationatSplinePoint _spline 0 "Local") "Local" true)))