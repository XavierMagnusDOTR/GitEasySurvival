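; BP_MapSelectionVolume is a trigger volume that switches the map, minimap and map render settings for the local player on entering or leaving it.
; On entry it passes its map sprite and clamp box to every BP_MapRenderActor and sets map and minimap availability through interface messages.
; On exit it clears and disables these, then hands over to an optional OutMapVolume.
; A helper derives and debug-draws the clamp box from the sprite and collision bounds.
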(event OnComponentBeginOverlap(CollisionComponent)
  (params (OverlappedComponent :type Primitive%20Component%20Object%20Reference) (OtherActor :type Actor%20Object%20Reference) (OtherComp :type Primitive%20Component%20Object%20Reference) (OtherBodyIndex :type Integer) (bFromSweep :type Boolean) (SweepResult :type Hit%20Result%20Structure%20%28by%20ref%29))
  ;[1 1 1] Begin and end overlap map selection collision.
  (Utilities|IsValid OtherActor
    (:Is%20Valid
      (bind _ascharacter (Utilities|Casting|CastToCharacter OtherActor))
      (bind _asplayer_controller (Utilities|Casting|CastToPlayerController (Pawn|GetController _ascharacter)))
      (if (Pawn|IsLocalPlayerController (Pawn|GetController _ascharacter))
        (CallFunction|UpdateMapforPlayer _asplayer_controller true)))))

(event OnComponentEndOverlap(CollisionComponent)
  (params (OverlappedComponent :type Primitive%20Component%20Object%20Reference) (OtherActor :type Actor%20Object%20Reference) (OtherComp :type Primitive%20Component%20Object%20Reference) (OtherBodyIndex :type Integer))
  ;[1 1 1] Begin and end overlap map selection collision.
  (Utilities|IsValid OtherActor
    (:Is%20Valid
      (bind _ascharacter (Utilities|Casting|CastToCharacter OtherActor))
      (bind _asplayer_controller (Utilities|Casting|CastToPlayerController (Pawn|GetController _ascharacter)))
      (if (Pawn|IsLocalPlayerController (Pawn|GetController _ascharacter))
        (CallFunction|UpdateMapforPlayer _asplayer_controller false)))))

(fn ConstructionScript)

(fn CheckMapEnabled
  (params (PlayerController :type Controller%20Object%20Reference) (CharacterEntered :type Boolean))
  ;[1 1 1] Check and disable map.
  (Utilities|IsValid PlayerController
    (:Is%20Valid
      (if CharacterEntered
        (Class|BPIPlayer|SetMapEnabledBPI(Message) PlayerController (Variables|Settings|GetMapEnabledInVolume))
        (else
          (Class|BPIPlayer|SetMapEnabledBPI(Message) PlayerController false))))))

(fn CheckMinimapEnabled
  (params (PlayerController :type Controller%20Object%20Reference) (CharacterEntered :type Boolean))
  ;[1 1 1] Check and disable minimap.
  (Utilities|IsValid PlayerController
    (:Is%20Valid
      (if CharacterEntered
        (Class|BPIPlayer|SetMinimapEnabledBPI(Message) PlayerController (Variables|Settings|GetMinimapEnabledInVolume))
        (else
          (Class|BPIPlayer|SetMinimapEnabledBPI(Message) PlayerController false))))))

(fn CheckRenderSettings
  (params (PlayerController :type Controller%20Object%20Reference) (CharacterEntered :type Boolean))
  ;[1 1 1] Check and show map sprite.
  (Utilities|IsValid PlayerController
    (:Is%20Valid
      (if (Variables|Settings|GetUpdateRenderSettings)
        (bind _outactors (Actor|GetAllActorsOfClass "/Game/EasySurvivalRPG/Blueprints/Misc/MapRenderSystem/BP_MapRenderActor.BP_MapRenderActor_C"))
        (for _array_element _outactors
          (if CharacterEntered
            (Default|SetRenderSettings _array_element (Variables|Settings|GetMapSprite) (Variables|Settings|GetClampRenderLocation) (Variables|Settings|GetClampBoxOrigin) (Variables|Settings|GetClampBoxExtent))
            (else
              (Default|ClearMapSelection _array_element))))))))

(fn UpdateMapforPlayer
  (params (PlayerController :type Player%20Controller%20Object%20Reference) (CharacterEntered :type Boolean))
  (bind _outmapvolume (Variables|Settings|GetOutMapVolume))
  ;[1 1 1] Update map selection for the player.
  (CallFunction|CheckRenderSettings PlayerController CharacterEntered)
  (CallFunction|CheckMapEnabled PlayerController CharacterEntered)
  (CallFunction|CheckMinimapEnabled PlayerController CharacterEntered)
  (if (not CharacterEntered)
    (Utilities|IsValid _outmapvolume
      (:Is%20Valid
        (CallFunction|UpdateMapforPlayer _outmapvolume PlayerController true)))))

(fn ClampSpriteBox
  (bind _collisioncomponent (Variables|Default|GetCollisionComponent))
  (bind _mapsprite (Variables|Settings|GetMapSprite))
  (bind (_origin _boxextent) (Collision|GetComponentBounds _collisioncomponent))
  (bind (_origin_2 _boxextent_2) (Collision|GetActorBounds _mapsprite false false))
  ;[1 1 1] Initialize clamp bound variables for selected map sprite.
  (Utilities|IsValid _mapsprite
    (:Is%20Valid
      (Variables|Settings|SetClampRenderLocation true)
      (Variables|Settings|SetClampBoxOrigin (Math|Vector|MakeVector (.x _origin_2) (.y _origin_2) (.z _origin)))
      (Variables|Settings|SetClampBoxExtent (Math|Vector|MakeVector (.x _boxextent_2) (.y _boxextent_2) (.z _boxextent)))
      (Settings|DrawClampBox))
    (:Is%20Not%20Valid
      (Variables|Settings|SetClampRenderLocation false))))

(fn DrawClampBox
  ;[1 1 1] Draw debug box for selected map sprite.
  (Rendering|Debug|DrawDebugBox (Variables|Settings|GetClampBoxOrigin) (Variables|Settings|GetClampBoxExtent) "(R=1.000000,G=0.000000,B=0.000000,A=1.000000)" "0, 0, 0" 5.0 0.0))