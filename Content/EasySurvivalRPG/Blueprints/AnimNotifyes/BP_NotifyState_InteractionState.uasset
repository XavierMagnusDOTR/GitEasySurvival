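; Anim notify state that flags an interaction state on the mesh's owner for the span of an animation window.
; Begin sets the chosen InteractionState true and End clears it, both through a Blueprint interface message to the owner.
; With UpdateByTick enabled, Tick re-sends the true state every frame.
; The notify name is built from the enum value, prefixed with InteractionState.
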(fn GetNotifyName
  (return (Utilities|String|Append "InteractionState_" (Utilities|String|EnumtoString (Variables|Default|GetInteractionState)))))

(fn ReceivedNotifyBegin
  (params (MeshComp :type Skeletal%20Mesh%20Component%20Object%20Reference) (Animation :type Anim%20Sequence%20Base%20Object%20Reference) (TotalDuration :type Float%20%28single-precision%29))
  ;[1 1 1] Set interaction state.
  (Class|BPICharacter|SetInteractionStateBPI(Message) (Components|GetOwner MeshComp) (Variables|Default|GetInteractionState) true)
  (return false))

(fn ReceivedNotifyEnd
  (params (MeshComp :type Skeletal%20Mesh%20Component%20Object%20Reference) (Animation :type Anim%20Sequence%20Base%20Object%20Reference))
  ;[1 1 1] Clear interaction state.
  (Class|BPICharacter|SetInteractionStateBPI(Message) (Components|GetOwner MeshComp) (Variables|Default|GetInteractionState) false)
  (return false))

(fn ReceivedNotifyTick
  (params (MeshComp :type Skeletal%20Mesh%20Component%20Object%20Reference) (Animation :type Anim%20Sequence%20Base%20Object%20Reference) (FrameDeltaTime :type Float%20%28single-precision%29))
  ;[1 1 1] Check and set interaction state by tick.
  (if (Variables|Default|GetUpdateByTick)
    (Class|BPICharacter|SetInteractionStateBPI(Message) (Components|GetOwner MeshComp) (Variables|Default|GetInteractionState) true)
    (return false)))